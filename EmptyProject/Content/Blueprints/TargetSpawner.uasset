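; Target spawner for a duck shooting-gallery style game, spawning moving Duck targets on random rows after a start delay.
; Tick reads score and rings left from the ScoreDisplay game mode, and a timer spawns a duck with that row's endpoints, speed and point value.
; When rings left drop to the hard-mode threshold, it plays a sound and switches to the bonus interval and harder speed.
; BeginPlay quits the game if the per-row arrays differ in length.
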(event EventBeginPlay
  (bind _spawnerarray (Variables|Default|GetSpawnerArray))
  (bind _rowvelocitymodifiers (Variables|Default|GetRowVelocityModifiers))
  (bind _returnvalue (Utilities|Array|Length _spawnerarray))
  (bind _returnvalue_2 (Utilities|Array|Length _rowvelocitymodifiers))
  (bind _asscore_display (Utilities|Casting|CastToScoreDisplay (Game|GetGameMode)))
  (Variables|Default|SetMaxRings (Variables|/Game/Blueprints/ScoreDisplay.ScoreDisplay_C|GetRings%20Left _asscore_display))
  (if (not (Math|Boolean|ANDBoolean (== (Utilities|Array|Length (Variables|Default|GetPointValues)) _returnvalue_2) (== _returnvalue_2 _returnvalue) (== _returnvalue (Utilities|Array|Length (Variables|Default|GetEndPointArray)))))
    (Class|VisualLoggerKismetLibrary|LogText "Error, array sizes [Start] and [End] do not equal each other" "Blueprint Log")
    (Game|QuitGame 0 "Quit")))

(event Collision|EventActorBeginOverlap
  (params (OtherActor :type Actor%20Object%20Reference)))

(event EventTick
  (params (DeltaSeconds :type Float%20%28single-precision%29))
  (bind _output_get (Variables|Default|SetCurrentTime (+ DeltaSeconds (Variables|Default|GetCurrentTime))))
  (if (>= _output_get (Variables|Default|GetStartSpawningDelay))
    (bind _asscore_display (Utilities|Casting|CastToScoreDisplay (Game|GetGameMode)))
    (CallFunction|MakeSpawnDecision (Variables|/Game/Blueprints/ScoreDisplay.ScoreDisplay_C|GetScore _asscore_display) (Variables|/Game/Blueprints/ScoreDisplay.ScoreDisplay_C|GetRings%20Left _asscore_display) (Variables|Default|GetCurrentTime) DeltaSeconds)))

(fn ConstructionScript)

(fn ChooseRandom
  (params (ChoiceArray :type Array%20of%20Actor%20Class%20References))
  (return (Utilities|Array|Get(acopy) ChoiceArray (Math|Random|RandomInteger (Utilities|Array|Length ChoiceArray)))))

(fn MakeSpawnDecision
  (params (Score :type Float%20%28single-precision%29) (RingsLeft :type Integer) (TotalTime :type Float%20%28single-precision%29) (DeltaTime :type Float%20%28single-precision%29))
  (bind _spawnerarray (Variables|Default|GetSpawnerArray))
  (bind _output_get (Variables|Default|SetSpawnTimer (+ (Variables|Default|GetSpawnTimer) DeltaTime)))
  (Class|VisualLoggerKismetLibrary|LogText "Spawn triggered!" "Blueprint Log")
  (if (>= _output_get (Variables|Default|GetSpawnInterval))
    (Variables|Default|SetSpawnTimer 0.0)
    (if (<= RingsLeft (Variables|Default|GetStartHardmodeAtRings))
      (if (== (Variables|Default|GetSpawnVelocityModifier) (Variables|Default|GetHarderSpawnVelocity))
        _
        (else
          (Audio|PlaySoundatLocation "/Game/Sounds/bonus-ducks_1.bonus-ducks_1" "0, 0, 0")
          (Variables|Default|SetSpawnInterval (Variables|Default|GetBonusInterval))
          (Variables|Default|SetSpawnVelocityModifier (Variables|Default|GetHarderSpawnVelocity))))
      (else
        (Variables|Default|SetSpawnVelocityModifier (Variables|Default|GetNormalSpawnVelocity))))
    (bind _output_get_2 (Variables|Default|SetRandomIntHolder (Math|Random|RandomInteger (Utilities|Array|Length _spawnerarray))))
    (bind _returnvalue (Game|SpawnActorfromClass "/Game/Blueprints/Duck.Duck_C" (Transformation|GetActorTransform (Utilities|Array|Get(acopy) _spawnerarray _output_get_2)) "AlwaysSpawn" 0 0))
    (Variables|/Game/Blueprints/Duck.Duck_C|SetStartPos _returnvalue (Transformation|GetActorTransform (Utilities|Array|Get(acopy) _spawnerarray _output_get_2)))
    (Variables|/Game/Blueprints/Duck.Duck_C|SetEndPos _returnvalue (Transformation|GetActorTransform (Utilities|Array|Get(acopy) (Variables|Default|GetEndPointArray) _output_get_2)))
    (Class|VisualLoggerKismetLibrary|LogText (Utilities|String|ToString(Float) (* (Utilities|Array|Get(acopy) (Variables|Default|GetRowVelocityModifiers) (Variables|Default|GetRandomIntHolder)) (* (Variables|Default|GetDifficulty) (Variables|Default|GetSpawnVelocityModifier)))) "Blueprint Log")
    (Variables|/Game/Blueprints/Duck.Duck_C|SetSpeed _returnvalue (* (Utilities|Array|Get(acopy) (Variables|Default|GetRowVelocityModifiers) (Variables|Default|GetRandomIntHolder)) (* (Variables|Default|GetDifficulty) (Variables|Default|GetSpawnVelocityModifier))))
    (Variables|/Game/Blueprints/Duck.Duck_C|SetPointValue _returnvalue (Utilities|Array|Get(acopy) (Variables|Default|GetPointValues) (Variables|Default|GetRandomIntHolder)))
    (Transformation|SetActorScale3D _returnvalue "2.000000,2.000000,2.000000")
    (Default|MovetoEnd _returnvalue)))