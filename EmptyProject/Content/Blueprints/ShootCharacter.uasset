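; Player shooter character with a limited aiming range that fires bullets in a ring-based score game.
; Turn and LookUp input is scaled, then applied only while accumulated yaw and pitch stay strictly inside their angle limits.
; Firing is cooldown-gated and asks the ScoreDisplay game mode to spawn bullets, then checks for game over a second later when no rings remain.
; PlayAgain restarts through that game mode.
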(event EventBeginPlay)

(event Collision|EventActorBeginOverlap
  (params (OtherActor :type Actor%20Object%20Reference)))

(event EventTick
  (params (DeltaSeconds :type Float%20%28single-precision%29))
  (Variables|Default|SetTimer (+ (Variables|Default|GetTimer) DeltaSeconds)))

(event Input|ActionEvents|InputActionFireGun
  (params (Key :type Key%20Structure :default "AnyKey"))
  (bind _returnvalue (Transformation|GetActorRotation))
  (:Pressed
    (if (>= (Variables|Default|GetTimer) (Variables|Default|GetDelay))
      (Variables|Default|SetTimer 0.0)
      (bind _asscore_display (Utilities|Casting|CastToScoreDisplay (Game|GetGameMode)))
      (Default|ShootBullet _asscore_display (Math|Transform|MakeTransform (+ (Transformation|GetActorLocation) (* (Math|Vector|GetForwardVector _returnvalue) 1e+02)) _returnvalue))
      (Utilities|FlowControl|Delay 1.0)
      (bind _asscore_display_2 (Utilities|Casting|CastToScoreDisplay (Game|GetGameMode)))
      (if (== (Variables|/Game/Blueprints/ScoreDisplay.ScoreDisplay_C|GetRings%20Left _asscore_display_2) 0)
        (Default|DisplayGameOver _asscore_display_2)))))

(event Input|ActionEvents|InputActionPlayAgain
  (params (Key :type Key%20Structure :default "AnyKey"))
  (:Pressed
    (bind _asscore_display (Utilities|Casting|CastToScoreDisplay (Game|GetGameMode)))
    (Default|RestartGame _asscore_display)))

(event Input|AxisEvents|InputAxisTurn
  (params (AxisValue :type Float%20%28single-precision%29))
  (bind _returnvalue (Math|Float|Clamp(Float) AxisValue -5.0 5.0))
  (bind _speedmod (Variables|Default|GetSpeedMod))
  (bind _returnvalue_2 (* _returnvalue _speedmod))
  (bind _insideclamp (CallFunction|ValidateMovement true _returnvalue_2 (Variables|Default|GetHorizontalCompositeClamp) (Variables|Default|GetMinAngleYaw) (Variables|Default|GetMaxAngleYaw)))
  (if _insideclamp
    (Pawn|Input|AddControllerYawInput _returnvalue_2)))

(event Input|AxisEvents|InputAxisLookUp
  (params (AxisValue :type Float%20%28single-precision%29))
  (bind _returnvalue (Math|Float|Clamp(Float) AxisValue -5.0 5.0))
  (bind _speedmod (Variables|Default|GetSpeedMod))
  (bind _returnvalue_2 (* _returnvalue _speedmod))
  (bind _insideclamp (CallFunction|ValidateMovement false _returnvalue_2 (Variables|Default|GetVerticalCompositeClamp) (Variables|Default|GetMinAnglePitch) (Variables|Default|GetMaxAnglePitch)))
  (if _insideclamp
    (Pawn|Input|AddControllerPitchInput _returnvalue_2)))

(event Input|MouseEvents|RightMouseButton
  (params (Key :type Key%20Structure :default "AnyKey"))
  (:Pressed
    (Variables|Default|SetRightMouseHeld true))
  (:Released
    (Variables|Default|SetRightMouseHeld false)))

(fn ConstructionScript)

(fn NormalizeSpeed
  (params (Value :type Float%20%28single-precision%29) (SpeedModifier :type Float%20%28single-precision%29))
  (return (* (/ Value (Math|Float|Absolute(Float) Value)) SpeedModifier)))

(fn ValidateMovement
  (params (IsHorizontal :type Boolean) (Speed :type Float%20%28single-precision%29) (Clamp :type Float%20%28single-precision%29) (MinAngle :type Float%20%28single-precision%29) (MaxAngle :type Float%20%28single-precision%29))
  (bind _composite (CallFunction|SetClampedComposite IsHorizontal Speed Clamp MinAngle MaxAngle))
  (return (Math|Float|InRange(Float) _composite MinAngle MaxAngle false false)))

(fn SetClampedComposite
  (params (IsHorizontal :type Boolean) (Speed :type Float%20%28single-precision%29) (Clamp :type Float%20%28single-precision%29) (MinAngle :type Float%20%28single-precision%29) (MaxAngle :type Float%20%28single-precision%29))
  (bind _returnvalue (+ Speed Clamp))
  (bind _returnvalue_2 (Math|Float|ClampAngle _returnvalue MinAngle MaxAngle))
  (if IsHorizontal
    (Variables|Default|SetHorizontalCompositeClamp _returnvalue_2)
    (else
      (Variables|Default|SetVerticalCompositeClamp _returnvalue_2)))
  (return _returnvalue_2))