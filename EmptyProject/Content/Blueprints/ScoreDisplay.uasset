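; ScoreDisplay manages the game's flow from title screen through play to game over, tracking score and remaining shots.
; BeginPlay hides screen debug messages, shows the title widget and plays music.
; The first ShootBullet call only swaps in the HUD; later calls spawn bullets while RingsLeft lasts, decrementing it.
; AddScore accumulates points, and DisplayGameOver shows the end screen and sets the flag that lets RestartGame reload SpawnTesting.
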(event EventBeginPlay
  (Development|ExecuteConsoleCommand "DISABLEALLSCREENMESSAGES")
  (Viewport|RemoveAllWidgets)
  (bind _returnvalue (UserInterface|CreateWidget "/Game/Blueprints/TitleScreen.TitleScreen_C"))
  (UserInterface|Viewport|AddtoViewport _returnvalue 0)
  (Audio|PlaySoundatLocation "/Game/Sounds/Merry-Go-Round_-_Super_Mario_64.Merry-Go-Round_-_Super_Mario_64" "0, 0, 0"))

(event EventTick
  (params (DeltaSeconds :type Float%20%28single-precision%29)))

(fn ConstructionScript)

(fn AddScore
  (params (Points :type Float%20%28single-precision%29))
  (bind _output_get (Variables|Default|SetScore (+ Points (Variables|Default|GetScore))))
  (return _output_get))

(fn ShootBullet
  (params (SpawnLocation :type Transform))
  (if (Variables|Default|GetFirstBulletFired)
    (if (> (Variables|Default|GetRings%20Left) 0)
      (Game|SpawnActorfromClass "/Game/Blueprints/Bullet.Bullet_C" SpawnLocation "Undefined" 0 0)
      (Variables|Default|SetRings%20Left (- (Variables|Default|GetRings%20Left) 1)))
    (else
      (Viewport|RemoveAllWidgets)
      (bind _returnvalue (UserInterface|CreateWidget "/Game/Blueprints/GameHUD.GameHUD_C"))
      (UserInterface|Viewport|AddtoViewport _returnvalue 0)
      (Variables|Default|SetFirstBulletFired true))))

(fn DisplayGameOver
  (Viewport|RemoveAllWidgets)
  (bind _returnvalue (UserInterface|CreateWidget "/Game/Blueprints/GameOverScreen.GameOverScreen_C"))
  (UserInterface|Viewport|AddtoViewport _returnvalue 0)
  (Variables|Default|SetGameOver true))

(fn RestartGame
  (if (Variables|Default|GetGameOver)
    (Game|OpenLevel(byName) "SpawnTesting")))