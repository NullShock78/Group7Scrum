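; Duck target actor that travels between two points and awards score when hit by a Bullet.
; MoveToEnd derives travel time from distance and Speed and sets the lifespan to just past it, while Tick lerps the position along the path.
; A bullet hit destroys the bullet, adds points through the ScoreDisplay game mode, then zeroes the point value and tips the duck over until its pitch check destroys it.
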(event Custom|FallDown
  (Variables|Default|SetPointValue 0)
  (Variables|Default|SetWasHit true))

(event Custom|MoveToEnd
  (bind _endpos (Variables|Default|GetEndPos))
  (bind _startpos (Variables|Default|GetStartPos))
  (bind _speed (Variables|Default|GetSpeed))
  (bind _location (Math|Transform|BreakTransform _endpos))
  (bind _location_2 (Math|Transform|BreakTransform _startpos))
  (bind _returnvalue (- _location _location_2))
  (bind _returnvalue_2 (Math|Vector|VectorLength _returnvalue))
  (bind _returnvalue_3 (/ _returnvalue_2 _speed))
  (Development|PrintString (Utilities|String|ToString(Float) _returnvalue_3))
  (Variables|Default|SetMoveDirection _returnvalue)
  (Actor|SetLifeSpan (+ _returnvalue_3 0.02))
  (Variables|Default|SetTT _returnvalue_3))

(event EventBeginPlay)

(event EventTick
  (params (DeltaSeconds :type Float%20%28single-precision%29))
  (bind _output_get (Variables|Default|SetTA (+ (Variables|Default|GetTA) DeltaSeconds)))
  (Transformation|SetActorLocation (Math|Vector|Lerp(Vector) (.Location (Math|Transform|BreakTransform (Variables|Default|GetStartPos))) (.Location (Math|Transform|BreakTransform (Variables|Default|GetEndPos))) (/ _output_get (Variables|Default|GetTT))) false false)
  (if (Variables|Default|GetWasHit)
    (Transformation|SetActorRotation (Math|Rotator|MakeRotfromZ (Math|Vector|RotateVectorAroundAxis (Transformation|GetActorUpVector) (* DeltaSeconds 2.7e+02) "0,1.000000, 0")))
    (if (>= (.Pitch (Math|Rotator|BreakRotator (Transformation|GetActorRotation))) 9e+01)
      (Actor|DestroyActor))))

(event Collision|EventHit
  (params (MyComp :type Primitive%20Component%20Object%20Reference) (Other :type Actor%20Object%20Reference) (OtherComp :type Primitive%20Component%20Object%20Reference) (bSelfMoved :type Boolean) (HitLocation :type Vector :default "0, 0, 0") (HitNormal :type Vector :default "0, 0, 0") (NormalImpulse :type Vector :default "0, 0, 0") (Hit :type Hit%20Result%20Structure%20%28by%20ref%29))
  (Class|VisualLoggerKismetLibrary|LogText "Overlap!" "DuckLog")
  (bind _asbullet (Utilities|Casting|CastToBullet Other))
  (Actor|DestroyActor _asbullet)
  (bind _asscore_display (Utilities|Casting|CastToScoreDisplay (Game|GetGameMode)))
  (Default|AddScore _asscore_display (Math|Conversions|ToFloat(Integer) (Variables|Default|GetPointValue)))
  (CallFunction|FallDown))

(fn ConstructionScript)